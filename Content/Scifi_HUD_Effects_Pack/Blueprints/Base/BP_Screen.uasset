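; BP_Screen is a screen actor from a sci-fi HUD effects pack that configures the material on its SMTerminal mesh.
; The Construction Script creates a dynamic material instance on the MaterialIndex slot and feeds it the ScaleX/Y and OffsetX/Y variables as scalar parameters.
; It has no active runtime logic, as the event graph holds only disabled default events.
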(event EventBeginPlay)

(event Collision|EventActorBeginOverlap
  (params (OtherActor :type Actor%20Object%20Reference)))

(event EventTick
  (params (DeltaSeconds :type Float%20%28single-precision%29)))

(fn ConstructionScript
  (bind _returnvalue (Rendering|Material|CreateDynamicMaterialInstance (Variables|Default|GetSM_Terminal) (Variables|Default|GetMaterialIndex) 0 "None" :!class /Script/Engine.PrimitiveComponent))
  (Rendering|Material|SetScalarParameterValue _returnvalue "ScaleX" (Variables|Default|GetScaleX) :!class /Script/Engine.MaterialInstanceDynamic)
  (Rendering|Material|SetScalarParameterValue _returnvalue "ScaleY" (Variables|Default|GetScaleY) :!class /Script/Engine.MaterialInstanceDynamic)
  (Rendering|Material|SetScalarParameterValue _returnvalue "OffsetX" (Variables|Default|GetOffsetX) :!class /Script/Engine.MaterialInstanceDynamic)
  (Rendering|Material|SetScalarParameterValue _returnvalue "OffsetY" (Variables|Default|GetOffsetY) :!class /Script/Engine.MaterialInstanceDynamic))