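; BP_tree_decoration is a decorative actor in the Synthwave city content with two palm tree static mesh components.
; Its construction script gives each palm an independent random yaw in 60-degree steps and a mesh picked at random from the RandomMesh array, up to the Max index.
; The randomization is unseeded, so results can change whenever construction reruns, and the event graph holds no active logic.
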(event EventBeginPlay)

(event Collision|EventActorBeginOverlap
  (params (OtherActor :type Actor%20Object%20Reference)))

(event EventTick
  (params (DeltaSeconds :type Float%20%28single-precision%29)))

(fn ConstructionScript
  (bind _max (Variables|Default|GetMax))
  (Transformation|SetRelativeRotation (Variables|Default|GetSM_palm_tree_01) (Math|Rotator|MakeRotator 0.0 0.0 (* (Math|Conversions|ToFloat(Integer) (Math|Random|RandomInteger 6)) 6e+01)) false false)
  (Transformation|SetRelativeRotation (Variables|Default|GetSM_palm_tree_02) (Math|Rotator|MakeRotator 0.0 0.0 (* (Math|Conversions|ToFloat(Integer) (Math|Random|RandomInteger 6)) 6e+01)) false false)
  ;[1 1 1] Randomize Mesh
  (Components|StaticMesh|SetStaticMesh (Variables|Default|GetSM_palm_tree_01) (Utilities|Array|Get(acopy) (Variables|Default|GetRandomMesh) (Math|Random|RandomIntegerinRange 0 _max)))
  (Components|StaticMesh|SetStaticMesh (Variables|Default|GetSM_palm_tree_02) (Utilities|Array|Get(acopy) (Variables|Default|GetRandomMesh) (Math|Random|RandomIntegerinRange 0 _max))))