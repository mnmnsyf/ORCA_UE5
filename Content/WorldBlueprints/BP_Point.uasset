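; BP_Point is a world point actor that shows different markers depending on whether it is a start or end point.
; RefreshStartEndState shows the end Niagara effect and bomb-time widget for end points, and the next-point widget for start points, using IsStart and IsEnd.
; SetTipsState toggles the next-point tip directly, while getters expose that tip's world location and the WBP_BombTime widget.
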(event EventBeginPlay)

(event Collision|EventActorBeginOverlap
  (params (OtherActor :type Actor%20Object%20Reference)))

(event EventTick
  (params (DeltaSeconds :type Float%20%28single-precision%29)))

(event EventSetTipsState
  (params (bShow :type Boolean))
  (Rendering|SetVisibility (Variables|Default|GetWidget_NextPoint) bShow false))

(event EventRefreshStartEndState
  (bind _returnvalue (Class|SpiderManTargetPoint|IsEnd))
  (Rendering|SetVisibility (Variables|Default|GetNiagara_End) _returnvalue false)
  (Rendering|SetVisibility (Variables|Default|GetWidget_BombTime) _returnvalue false)
  (Rendering|SetVisibility (Variables|Default|GetWidget_NextPoint) (Class|SpiderManTargetPoint|IsStart) false))

(fn ConstructionScript)

(fn GetTipActorLocation
  (return (Transformation|GetWorldLocation (Variables|Default|GetWidget_NextPoint))))

(fn GetBombTimeUI
  (bind _aswbp_bomb_time (Utilities|Casting|CastToWBP_BombTime (UserInterface|GetWidget (Variables|Default|GetWidget_BombTime))))
  (return _aswbp_bomb_time))